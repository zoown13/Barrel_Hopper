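; HUD for the Barrel Hopper game that shows the player's attempt count and a game-over message.
; Each DrawHUD call checks GameWon to choose between DrawInGame and DrawEndGame.
; In play, the attempt count sits near top center; the end screen adds restart and quit key prompts around mid-screen.
; Text is drawn directly with DrawText, positioned from viewport and measured text sizes.
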(event EventBeginPlay)

(event Collision|EventActorBeginOverlap
  (params (OtherActor :type Actor%20Object%20Reference)))

(event EventTick
  (params (DeltaSeconds :type Float%20%28single-precision%29)))

(event EventDrawHUD
  (params (SizeX :type Integer) (SizeY :type Integer))
  (if (Variables|Default|GetGameWon)
    (CallFunction|DrawEndGame)
    (else
      (CallFunction|DrawinGame))))

(fn ConstructionScript)

(fn DrawinGame
  (HUD|DrawText (Utilities|String|ToString(Float) (Variables|Default|GetPlayerAttempt)) "(R=0.863157,G=0.658375,B=0.046665,A=1.000000)" (- (* (.X (Math|Vector2D|BreakVector2D (Viewport|GetViewportSize))) 0.5) (* (.OutWidth (Class|HUD|GetTextSize "111" (Variables|Default|GetScreenFont) 1.0)) 0.5)) 0.0 (Variables|Default|GetScreenFont) 1.0 false))

(fn DrawEndGame
  (bind _returnvalue (Viewport|GetViewportSize))
  (bind _screenfont (Variables|Default|GetScreenFont))
  (bind (_x _y) (Math|Vector2D|BreakVector2D _returnvalue))
  (bind (_outwidth _outheight) (Class|HUD|GetTextSize "Press R to restart or X to Quit!" _screenfont 1.0))
  (HUD|DrawText (Utilities|String|Append "Game Over!! 
" (Utilities|String|ToString(Float) (Variables|Default|GetPlayerAttempt)) " 
" "Press R to restart or X to Quit!") "(R=0.863157,G=0.708376,B=0.045186,A=1.000000)" (- (* _x 0.5) (* _outwidth 0.0)) (- (* _y 0.5) (* (* _outheight 3.0) 0.5)) (Variables|Default|GetScreenFont) 1.0 false))